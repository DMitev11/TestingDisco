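; Prototype player car pawn with simple arcade driving that moves without physics forces or collision sweeps.
; Enhanced Input adds forward acceleration to a velocity vector and yaws the root for steering.
; Tick damps velocity, offsets the root, snaps its height to a downward trace from CameraViewpoint and prints a debug KPH readout.
; Number keys 1–4 nudge the level's BP_Camera through CamTool.
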(event Input|EnhancedActionEvents|EnhancedInputActionIA_Forward
  (params (ActionValue :type Float%20%28double-precision%29) (ElapsedSeconds :type Float%20%28double-precision%29) (TriggeredSeconds :type Float%20%28double-precision%29) (InputAction :type Input%20Action%20Object%20Reference :default "/Game/Input/IA_Forward.IA_Forward"))
  (Variables|Default|SetVelocity (+ (Variables|Default|GetVelocity) (* ActionValue (Math|Vector|GetForwardVector (Variables|Default|GetDefaultSceneRoot)) (Variables|Default|GetAccel) (* (Utilities|Time|GetWorldDeltaSeconds) 1.2e+02)))))

(event Input|EnhancedActionEvents|EnhancedInputActionIA_Left
  (params (ActionValue :type Float%20%28double-precision%29) (ElapsedSeconds :type Float%20%28double-precision%29) (TriggeredSeconds :type Float%20%28double-precision%29) (InputAction :type Input%20Action%20Object%20Reference :default "/Game/Input/IA_Left.IA_Left"))
  (Transformation|AddRelativeRotation (Variables|Default|GetDefaultSceneRoot) (Math|Rotator|MakeRotator 0.0 0.0 (* ActionValue -1.0 (* (Utilities|Time|GetWorldDeltaSeconds) 1.2e+02))) false false))

(event EventBeginPlay
  (bind _asplayer_controller (Utilities|Casting|CastToPlayerController (Pawn|GetController)))
  (Input|AddMappingContext (PlayerController|LocalPlayerSubsystems|GetEnhancedInputLocalPlayerSubsystem _asplayer_controller) "/Game/Input/MC_Cartest.MC_Cartest" 0 "(bIgnoreAllPressedKeysUntilRelease=True,bForceImmediately=False,bNotifyUserSettings=False)")
  (bind _returnvalue (Actor|GetActorOfClass "/Game/Prototypes/BP_Camera.BP_Camera_C"))
  (Variables|Default|SetCamRef _returnvalue))

(event EventTick
  (params (DeltaSeconds :type Float%20%28single-precision%29))
  (bind _cameraviewpoint (Variables|Default|GetCameraViewpoint))
  (bind _defaultsceneroot (Variables|Default|GetDefaultSceneRoot))
  (bind _returnvalue (Transformation|GetWorldLocation _defaultsceneroot))
  (bind _returnvalue_2 (Transformation|GetWorldLocation _cameraviewpoint))
  (Variables|Default|SetVelocity (Math|Vector|Lerp(Vector) (Variables|Default|GetVelocity) "0, 0, 0" 0.025))
  (Transformation|AddWorldOffset (Variables|Default|GetDefaultSceneRoot) (Variables|Default|GetVelocity) false false)
  (Development|PrintString (Utilities|String|Append "KPH: " (Utilities|String|ToString(Float) (+ (Math|Float|Sqrt (Math|Float|Square (.X (Math|Vector|BreakVector (Variables|Default|GetVelocity))))) (Math|Float|Sqrt (Math|Float|Square (.Y (Math|Vector|BreakVector (Variables|Default|GetVelocity))))) (Math|Float|Sqrt (Math|Float|Square (.Z (Math|Vector|BreakVector (Variables|Default|GetVelocity)))))))) true true "(R=0.000000,G=0.660000,B=1.000000,A=1.000000)" 0.0)
  (bind _outhit (Collision|LineTraceByChannel _returnvalue_2 (- _returnvalue_2 "0.000000,0.000000,2000.000000") "TraceTypeQuery1" false 0 "None"))
  (Transformation|SetWorldLocation _defaultsceneroot (Math|Vector|MakeVector (.x _returnvalue) (.y _returnvalue) (.z (.location _outhit))) false false))

(event Input|KeyboardEvents|1
  (params (Key :type Key%20Structure :default "None"))
  (:Pressed
    (Default|CamTool (Variables|Default|GetCamRef) 0.0 0.5)))

(event Input|KeyboardEvents|2
  (params (Key :type Key%20Structure :default "None"))
  (:Pressed
    (Default|CamTool (Variables|Default|GetCamRef) 0.0 -0.5)))

(event Input|KeyboardEvents|3
  (params (Key :type Key%20Structure :default "None"))
  (:Pressed
    (Default|CamTool (Variables|Default|GetCamRef) 0.5 0.0)))

(event Input|KeyboardEvents|4
  (params (Key :type Key%20Structure :default "None"))
  (:Pressed
    (Default|CamTool (Variables|Default|GetCamRef) -0.5 0.0)))

(fn ConstructionScript)