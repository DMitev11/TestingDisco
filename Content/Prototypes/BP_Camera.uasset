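; Prototype follow camera that takes over the view on BeginPlay and keeps a fixed offset from BP_ProtPlayer.
; On BeginPlay or Adjustcam, it traces along the camera's forward vector, moves the player to the hit location and stores the camera-to-player offset.
; Tick reapplies that offset to the player's position to move the camera actor.
; CamTool adjusts either pitch or yaw, keeping roll at zero.
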(event Custom|Attach%20Cam%20to%20vehicle
  (Transformation|SetActorLocation (+ (Transformation|GetWorldLocation (Variables|/Script/Engine.Actor|GetRootComponent (Variables|Default|GetPlayer%20ref))) (Variables|Default|GetDeltaLoc)) false false))

(event Custom|Adjust%20cam
  (bind _camera (Variables|Default|GetCamera))
  (bind _player_ref (Variables|Default|GetPlayer%20ref))
  (bind _returnvalue (Transformation|GetWorldLocation _camera))
  (bind _rootcomponent (Variables|/Script/Engine.Actor|GetRootComponent _player_ref))
  (bind _outhit (Collision|LineTraceByChannel _returnvalue (+ _returnvalue (* (Math|Vector|GetForwardVector (Transformation|GetWorldRotation _camera)) 9e+03)) "TraceTypeQuery1" false 0 "Persistent"))
  (Transformation|SetWorldLocation _rootcomponent (.location _outhit) false false)
  (Variables|Default|SetDeltaLoc (- (Transformation|GetWorldLocation (Variables|Default|GetCamera)) (Transformation|GetWorldLocation _rootcomponent))))

(event Custom|CamTool
  (params (Y :type Float%20%28double-precision%29) (Z :type Float%20%28double-precision%29))
  (bind _camera (Variables|Default|GetCamera))
  (bind _camera_2 (Variables|Default|GetCamera))
  (bind _returnvalue (Transformation|GetWorldRotation _camera))
  (bind _returnvalue_2 (Transformation|GetWorldRotation _camera))
  (if (== Y 0.0)
    (Transformation|SetWorldRotation _camera_2 (Math|Rotator|MakeRotator 0.0 (.pitch _returnvalue_2) (.yaw (Math|Rotator|CombineRotators _returnvalue (Math|Rotator|MakeRotator 0.0 0.0 Z)))) false false)
    (else
      (Transformation|SetWorldRotation _camera_2 (Math|Rotator|MakeRotator 0.0 (.pitch (Math|Rotator|CombineRotators _returnvalue (Math|Rotator|MakeRotator 0.0 Y 0.0))) (.yaw _returnvalue_2)) false false))))

(event EventBeginPlay
  (bind _camera (Variables|Default|GetCamera))
  (bind _returnvalue (Transformation|GetWorldLocation _camera))
  (Variables|Default|SetbFindCameraComponentWhenViewTarget true)
  (Game|Player|SetViewTargetwithBlend (Game|GetPlayerController (Variables|/Script/Engine.Pawn|GetPlayerState (Game|Player|GetPlayerPawn 0))) self 0.0 "VTBlend_Linear" 0.0 false)
  (bind _returnvalue_2 (Actor|GetActorOfClass "/Game/Prototypes/BP_ProtPlayer.BP_ProtPlayer_C"))
  (Variables|Default|SetPlayer%20ref _returnvalue_2)
  (bind _outhit (Collision|LineTraceByChannel _returnvalue (+ _returnvalue (* (Math|Vector|GetForwardVector (Transformation|GetWorldRotation _camera)) 9e+03)) "TraceTypeQuery1" false 0 "Persistent"))
  (Transformation|SetWorldLocation (Variables|/Script/Engine.Actor|GetRootComponent (Variables|Default|GetPlayer%20ref)) (.location _outhit) false false)
  (Variables|Default|SetDeltaLoc (- (Transformation|GetWorldLocation (Variables|Default|GetCamera)) (Transformation|GetWorldLocation (Variables|/Script/Engine.Actor|GetRootComponent (Variables|Default|GetPlayer%20ref))))))

(event Collision|EventActorBeginOverlap
  (params (OtherActor :type Actor%20Object%20Reference)))

(event EventTick
  (params (DeltaSeconds :type Float%20%28single-precision%29))
  (Utilities|FlowControl|Sequence
    (:then_0
      (Utilities|FlowControl|DoOnce false
        (:Completed
          (Utilities|FlowControl|Delay 0.2))))
    (:then_1
      (CallFunction|AttachCamtoVehicle))))

(fn ConstructionScript)