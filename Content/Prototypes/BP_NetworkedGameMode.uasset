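; Prototype game mode that hosts or joins a SteamCore Pro online session when play begins.
; It searches for sessions with the server name "Testing Disco" and calls a session node with that name, apparently to create one, if at most one is found.
; With more results, it runs a second, unfiltered search and joins its first result through the first player controller.
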(event EventBeginPlay
  (bind _results (|FindSteamCoreProSessions (Utilities|Map|MakeMap "ServerName" (Class|SteamUtilities|MakeSearchString "Testing Disco")) 50 false "Listen" false false 1e+01)
    (:then
      (if (>= 1 (Utilities|Array|Length _results))
        (|SteamCoreProSession 0 "Testing Disco" 5 false true true true false false false true true 1e+01)
        (else
          (bind _results_2 (|FindSteamCoreProSessions 0 50 false "Listen" false false 1e+01)
            (:OnCallback
              (|JoinSession (Game|GetPlayerController 0) (.result (Utilities|Array|Get(acopy) _results_2))))))))))

(fn ConstructionScript)